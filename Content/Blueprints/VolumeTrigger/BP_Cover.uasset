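; BP_Cover is a cover volume that marks the player character and NPCs as safe while they overlap its Box.
; Begin and end overlap cast the other actor to BP_TopDownCharacter, BP_NPC or BP_NPC2, then set or clear InSafe and show or hide the Cube mesh.
; Occupants are not counted, so any one leaving hides the Cube.
; The material-swap nodes never run.
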(event OnComponentBeginOverlap(Box)
  (params (OverlappedComponent :type Primitive%20Component%20Object%20Reference) (OtherActor :type Actor%20Object%20Reference) (OtherComp :type Primitive%20Component%20Object%20Reference) (OtherBodyIndex :type Integer) (bFromSweep :type Boolean) (SweepResult :type Hit%20Result%20Structure%20%28by%20ref%29))
  (bind _asbp_top_down_character (Utilities|Casting|CastToBP_TopDownCharacter OtherActor)
    (:then
      (Default|SetinSafe _asbp_top_down_character true)
      (Rendering|SetVisibility (Variables|Default|GetCube) true false))
    (:CastFailed
      (bind _asbp_npc (Utilities|Casting|CastToBP_NPC OtherActor)
        (:then
          (Default|SetinSafe _asbp_npc true)
          (Rendering|SetVisibility (Variables|Default|GetCube) true false))
        (:CastFailed
          (bind _asbp_npc2 (Utilities|Casting|CastToBP_NPC2 OtherActor))
          (Default|SetinSafe _asbp_npc2 true)
          (Rendering|SetVisibility (Variables|Default|GetCube) true false))))))

(event OnComponentEndOverlap(Box)
  (params (OverlappedComponent :type Primitive%20Component%20Object%20Reference) (OtherActor :type Actor%20Object%20Reference) (OtherComp :type Primitive%20Component%20Object%20Reference) (OtherBodyIndex :type Integer))
  (bind _asbp_top_down_character (Utilities|Casting|CastToBP_TopDownCharacter OtherActor)
    (:then
      (Default|SetinSafe _asbp_top_down_character false)
      (Rendering|SetVisibility (Variables|Default|GetCube) false false))
    (:CastFailed
      (bind _asbp_npc (Utilities|Casting|CastToBP_NPC OtherActor)
        (:then
          (Default|SetinSafe _asbp_npc false)
          (Rendering|SetVisibility (Variables|Default|GetCube) false false))
        (:CastFailed
          (bind _asbp_npc2 (Utilities|Casting|CastToBP_NPC2 OtherActor))
          (Default|SetinSafe _asbp_npc2 false)
          (Rendering|SetVisibility (Variables|Default|GetCube) false false))))))

(event EventBeginPlay)

(event Collision|EventActorBeginOverlap
  (params (OtherActor :type Actor%20Object%20Reference)))

(event EventTick
  (params (DeltaSeconds :type Float%20%28single-precision%29)))

(fn ConstructionScript)
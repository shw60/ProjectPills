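; Trap actor for the player and two NPC types that randomly becomes a dropping-block or explosive trap at BeginPlay.
; Entering the box flags the character as trapped and reveals either a physics-driven Cube or a Plane with a repeating countdown timer.
; The countdown ends in an explosion that kills that character if still flagged; leaving the box clears the flag.
; The Cube's hit kills only the player.
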(event OnComponentBeginOverlap(Box)
  (params (OverlappedComponent :type Primitive%20Component%20Object%20Reference) (OtherActor :type Actor%20Object%20Reference) (OtherComp :type Primitive%20Component%20Object%20Reference) (OtherBodyIndex :type Integer) (bFromSweep :type Boolean) (SweepResult :type Hit%20Result%20Structure%20%28by%20ref%29))
  (bind _asbp_top_down_character (Utilities|Casting|CastToBP_TopDownCharacter OtherActor)
    (:then
      (Default|SetinTrap _asbp_top_down_character true)
      (switch Utilities|FlowControl|Switch|SwitchonETrapType (Variables|Default|GetCurrentTrapType)
        (:NewEnumerator0
          (Rendering|SetVisibility (Variables|Default|GetCube) true false)
          (Physics|SetSimulatePhysics (Variables|Default|GetCube) true))
        (:NewEnumerator1
          (Rendering|SetVisibility (Variables|Default|GetPlane) true false)
          (bind _returnvalue (Utilities|Time|SetTimerbyEvent (delegate Custom|ExplosiveTimerEvent) 1.0 true))
          (Variables|Default|SetExplosiveTimer _returnvalue))))
    (:CastFailed
      (bind _asbp_npc (Utilities|Casting|CastToBP_NPC OtherActor)
        (:then
          (Default|SetinTrap _asbp_npc true)
          (switch Utilities|FlowControl|Switch|SwitchonETrapType (Variables|Default|GetCurrentTrapType)
            (:NewEnumerator0
              (Rendering|SetVisibility (Variables|Default|GetCube) true false)
              (Physics|SetSimulatePhysics (Variables|Default|GetCube) true))
            (:NewEnumerator1
              (Rendering|SetVisibility (Variables|Default|GetPlane) true false)
              (bind _returnvalue_2 (Utilities|Time|SetTimerbyEvent (delegate Custom|ExplosiveTimerEvent1) 1.0 true))
              (Variables|Default|SetExplosiveTimer _returnvalue_2))))
        (:CastFailed
          (bind _asbp_npc2 (Utilities|Casting|CastToBP_NPC2 OtherActor))
          (Default|SetinTrap _asbp_npc2 true)
          (switch Utilities|FlowControl|Switch|SwitchonETrapType (Variables|Default|GetCurrentTrapType)
            (:NewEnumerator0
              (Rendering|SetVisibility (Variables|Default|GetCube) true false)
              (Physics|SetSimulatePhysics (Variables|Default|GetCube) true))
            (:NewEnumerator1
              (Rendering|SetVisibility (Variables|Default|GetPlane) true false)
              (bind _returnvalue_3 (Utilities|Time|SetTimerbyEvent (delegate Custom|ExplosiveTimerEvent2) 1.0 true))
              (Variables|Default|SetExplosiveTimer _returnvalue_3))))))))

(event OnComponentHit(Cube)
  (params (HitComponent :type Primitive%20Component%20Object%20Reference) (OtherActor :type Actor%20Object%20Reference) (OtherComp :type Primitive%20Component%20Object%20Reference) (NormalImpulse :type Vector :default "0, 0, 0") (Hit :type Hit%20Result%20Structure%20%28by%20ref%29))
  (bind _asbp_top_down_character (Utilities|Casting|CastToBP_TopDownCharacter OtherActor)
    (:then
      (Default|ForceKill _asbp_top_down_character))
    (:CastFailed
      (Utilities|Casting|CastToBP_NPC2 OtherActor))))

(event OnComponentEndOverlap(Box)
  (params (OverlappedComponent :type Primitive%20Component%20Object%20Reference) (OtherActor :type Actor%20Object%20Reference) (OtherComp :type Primitive%20Component%20Object%20Reference) (OtherBodyIndex :type Integer))
  (bind _asbp_top_down_character (Utilities|Casting|CastToBP_TopDownCharacter OtherActor)
    (:then
      (Default|SetinTrap _asbp_top_down_character false))
    (:CastFailed
      (bind _asbp_npc (Utilities|Casting|CastToBP_NPC OtherActor)
        (:then
          (Default|SetinTrap _asbp_npc false))
        (:CastFailed
          (bind _asbp_npc2 (Utilities|Casting|CastToBP_NPC2 OtherActor))
          (Default|SetinTrap _asbp_npc2 false))))))

(event Custom|ExplosiveTimerEvent1
  (bind _result (Math|Integer|DecrementInt (Variables|Default|GetExplsiveWaitTime))
    (:%20%20
      (if (<= _result 0)
        (Effects|SpawnEmitteratLocation "/Game/Another/InfinityBladeEffects/Effects/FX_Monsters/FX_Monster_Gruntling/Bomber/P_BomberExplode.P_BomberExplode" (Transformation|GetWorldLocation (Variables|Default|GetPlane)) "0, 0, 0" "2.000000,2.000000,2.000000")
        (Utilities|Time|ClearandInvalidateTimerbyHandle (Variables|Default|GetExplosiveTimer))
        (Rendering|SetVisibility (Variables|Default|GetPlane) false false)
        (if (Variables|/Game/Blueprints/Character/NonPlayerbleCharacter/BP_NPC.BP_NPC_C|GetIsInTrap (stale OnComponentBeginOverlap(Box) _asbp_npc))
          (Default|ForceKill (stale OnComponentBeginOverlap(Box) _asbp_npc)))))))

(event Custom|ExplosiveTimerEvent
  (bind _result (Math|Integer|DecrementInt (Variables|Default|GetExplsiveWaitTime))
    (:%20%20
      (if (<= _result 0)
        (Effects|SpawnEmitteratLocation "/Game/Another/InfinityBladeEffects/Effects/FX_Monsters/FX_Monster_Gruntling/Bomber/P_BomberExplode.P_BomberExplode" (Transformation|GetWorldLocation (Variables|Default|GetPlane)) "0, 0, 0" "3.000000,3.000000,3.000000")
        (Utilities|Time|ClearandInvalidateTimerbyHandle (Variables|Default|GetExplosiveTimer))
        (Rendering|SetVisibility (Variables|Default|GetPlane) false false)
        (if (Variables|/Game/Blueprints/Character/PlayerCharacter/BP_TopDownCharacter.BP_TopDownCharacter_C|GetIsInTrap (stale OnComponentBeginOverlap(Box) _asbp_top_down_character))
          (Default|ForceKill (stale OnComponentBeginOverlap(Box) _asbp_top_down_character)))))))

(event Custom|ExplosiveTimerEvent2
  (bind _result (Math|Integer|DecrementInt (Variables|Default|GetExplsiveWaitTime))
    (:%20%20
      (if (<= _result 0)
        (Effects|SpawnEmitteratLocation "/Game/Another/InfinityBladeEffects/Effects/FX_Monsters/FX_Monster_Gruntling/Bomber/P_BomberExplode.P_BomberExplode" (Transformation|GetWorldLocation (Variables|Default|GetPlane)) "0, 0, 0" "2.000000,2.000000,2.000000")
        (Utilities|Time|ClearandInvalidateTimerbyHandle (Variables|Default|GetExplosiveTimer))
        (Rendering|SetVisibility (Variables|Default|GetPlane) false false)
        (if (Variables|/Game/Blueprints/Character/NonPlayerbleCharacter/BP_NPC2.BP_NPC2_C|GetIsInTrap (stale OnComponentBeginOverlap(Box) _asbp_npc2))
          (Default|ForceKill (stale OnComponentBeginOverlap(Box) _asbp_npc2)))))))

(event EventBeginPlay
  (Rendering|SetVisibility (Variables|Default|GetCube) false false)
  (Physics|SetSimulatePhysics (Variables|Default|GetCube) false)
  (Rendering|SetVisibility (Variables|Default|GetPlane) false false)
  ;[1 1 1] 함정 타입 랜덤 설정
  (CallFunction|InitTrapType))

(event Collision|EventActorBeginOverlap
  (params (OtherActor :type Actor%20Object%20Reference)))

(event EventTick
  (params (DeltaSeconds :type Float%20%28single-precision%29)))

(fn ConstructionScript)

(fn InitTrapType
  (Utilities|Array|AddUnique (Variables|Default|Gettraptypes) "NewEnumerator0")
  (Utilities|Array|AddUnique (Variables|Default|Gettraptypes) "NewEnumerator1")
  (bind _output_get (Variables|Default|SetCurrentTrapType (.OutItem (Utilities|Array|Random (Variables|Default|Gettraptypes)))))
  (Development|PrintString (Utilities|String|EnumtoString _output_get)))
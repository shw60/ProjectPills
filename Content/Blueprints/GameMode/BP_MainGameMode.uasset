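; Main game mode that runs a timed round through ready, playing and result states.
; Ready shows the title widget; playing hides it, possesses the placed top-down character and spawns IT1/IT2 actors at spawn points, stepping IT2 rotation speed.
; A looping one-second timer updates the controller's countdown and, after time-out, finish-zone arrival or death, waits briefly before entering result.
; Result clears the timer and reloads the current level.
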(event Custom|CustomEvent
  (bind _playerconstroller (Variables|Default|GetPlayerConstroller))
  (Utilities|IsValid _playerconstroller
    (:Is%20Valid
      (Default|SetMainTimer _playerconstroller (Utilities|String|ToString(Text) (Utilities|Text|FormatText "RemainTime : {T}" (CallFunction|FormatMinSecond (Variables|Default|GetPlayTime)))))
      (Math|Integer|DecrementInt (Variables|Default|GetPlayTime)
        (:%20%20
          (if (Math|Boolean|ORBoolean (<= (Variables|Default|GetPlayTime) 0) (Variables|/Game/Blueprints/Character/PlayerCharacter/BP_TopDownCharacter.BP_TopDownCharacter_C|GetIsInFinishZone (Variables|Default|GetPlayer)) (Variables|/Game/Blueprints/Character/PlayerCharacter/BP_TopDownCharacter.BP_TopDownCharacter_C|GetIsDead (Variables|Default|GetPlayer)))
            (Utilities|FlowControl|Delay 2.0)
            (CallFunction|SetCurrentGameState "NewEnumerator2")))))))

(event Custom|SetCurrentGameState
  (params (GameState :type EPlayState%20Enum :default "NewEnumerator0"))
  (Variables|Default|SetCurrentGameState GameState)
  (switch Utilities|FlowControl|Switch|SwitchonEPlayState (Variables|Default|GetCurrentGameState)
    (:NewEnumerator1
      (Widget|SetVisibility (Variables|Default|GetTitleWidget) "Hidden")
      (CallFunction|SpawnPlayer)
      (CallFunction|SpawnIT)
      (CallFunction|SpawnIT2)
      (bind _returnvalue (Utilities|Time|SetTimerbyEvent (delegate Custom|CustomEvent) 1.0 true))
      (Variables|Default|SetMainTimerHandle _returnvalue))
    (:NewEnumerator2
      ;[1 1 1] 타이머 정지
      (Utilities|Time|ClearandInvalidateTimerbyHandle (Variables|Default|GetMainTimerHandle))
      (bind _returnvalue_2 (Game|GetCurrentLevelName true))
      (Game|OpenLevel(byName) (Utilities|String|StringToName _returnvalue_2)))))

(event EventBeginPlay
  (switch Utilities|FlowControl|Switch|SwitchonEPlayState (Variables|Default|GetCurrentGameState)
    (:NewEnumerator0
      (bind _returnvalue (UserInterface|CreateWidget "/Game/UI/WidgetBP_GameTitle.WidgetBP_GameTitle_C"))
      (bind _output_get (Variables|Default|SetTitleWidget _returnvalue))
      (UserInterface|Viewport|AddtoViewport _output_get 0))))

(event EventTick
  (params (DeltaSeconds :type Float%20%28single-precision%29)))

(event EventPostLogin
  (params (NewPlayer :type Player%20Controller%20Object%20Reference))
  (bind _asbp_main_player_controller (Utilities|Casting|CastToBP_MainPlayerController NewPlayer))
  (Variables|Default|SetPlayerConstroller _asbp_main_player_controller))

(fn ConstructionScript)

(fn FormatMinSecond
  (params (Sec :type Integer))
  (bind _returnvalue (/ Sec 60))
  (bind _returnvalue_2 (Math|Integer|%(Integer) Sec 60))
  ;[1 1 1] 남은 시간이 1분 이상
  (if (== _returnvalue 0)
    _
    (else
      (LocalVariables|SetText (Utilities|String|Append (Utilities|String|ToString(Integer) _returnvalue) "'"))))
  ;[1 1 1] 1분 이하
  (if (not (== _returnvalue_2 0))
    (bind _output_get (LocalVariables|SetText (Utilities|String|Append (LocalVariables|GetText) (Utilities|String|ToString(Integer) _returnvalue_2) "\"")))
    (return (Utilities|Text|ToText(String) _output_get))))

(fn SpawnIT
  (bind _outactors (Actor|GetAllActorsOfClass "/Game/Blueprints/VolumeTrigger/BP_IT_SpawnPoint.BP_IT_SpawnPoint_C"))
  (for _array_element _outactors
    (Game|SpawnActorfromClass "/Game/Blueprints/Character/Doll/BP_IT1.BP_IT1_C" (Transformation|GetActorTransform _array_element) "Undefined" 0 0)))

(fn SpawnPlayer
  (bind _returnvalue (Actor|GetActorOfClass "/Game/Blueprints/Character/PlayerCharacter/BP_TopDownCharacter.BP_TopDownCharacter_C"))
  (bind _output_get (Variables|Default|SetPlayer _returnvalue))
  (Pawn|Possess (Game|GetPlayerController 0) _output_get))

(fn SpawnIT2
  (bind _index (LocalVariables|GetIndex))
  (bind _outactors (Actor|GetAllActorsOfClass "/Game/Blueprints/VolumeTrigger/BP_IT2_SpawnPoint.BP_IT2_SpawnPoint_C"))
  (for (_array_element _array_index) _outactors
    (bind _returnvalue (Game|SpawnActorfromClass "/Game/Blueprints/Character/Doll/BP_IT2.BP_IT2_C" (Transformation|GetActorTransform _array_element) "Undefined" 0 0))
    (if (== _array_index _index)
      (Default|SetIT _returnvalue _index (LocalVariables|GetRotationSpeed))
      (Math|Integer|IncrementInt (LocalVariables|GetIndex)
        (:%20%20
          (LocalVariables|SetRotationSpeed (+ (LocalVariables|GetRotationSpeed) -8e+01)))))))
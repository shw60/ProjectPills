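; BP_MainPlayerController is a player controller that shows the main timer widget and stores the play time.
; On BeginPlay it creates Widget_BP_MainTimer and adds it to the viewport, and its SetMainTimer event writes the given time to MainPlayTime.
; A disconnected chain, which never runs, would advance BP_MainGameMode from its first game state to the next once and set IsGameStart.
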(event Custom|SetMainTimer
  (params (Time :type String))
  (Variables|Default|SetMainPlayTime Time))

(event EventBeginPlay
  (bind _self self)
  (bind _returnvalue (UserInterface|CreateWidget "/Game/UI/Widget_BP_MainTimer.Widget_BP_MainTimer_C" _self _self))
  (UserInterface|Viewport|AddtoViewport _returnvalue 0))

(event EventTick
  (params (DeltaSeconds :type Float%20%28single-precision%29)))

(event Input|ActionEvents|InputActionMove
  (params (Key :type Key%20Structure :default "None")))

(fn ConstructionScript)
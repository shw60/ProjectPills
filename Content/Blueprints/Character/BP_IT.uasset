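; BP_IT is the Squid Game doll that acts as "it", turning its head back and forth at random intervals.
; Tick feeds a random 2–6 second Delay, which works as a repeating timer that calls Rotate180.
; A FlipFlop there alternates between the StopTiming and GoTiming timelines, each driving the head mesh's relative yaw.
; An actor-rotation node marked as temporary logic is left unconnected.
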(event Custom|Rotate180
  (Utilities|FlowControl|FlipFlop
    (:A
      ;[1 1 1] 회전 타이밍
      (bind _rotation (Timeline|StopTiming PlayFromStart)
        (:Update
          (Transformation|SetRelativeRotation (Variables|Default|GetsquidGame_Doll_squidGameDoll_02_kepala) (Math|Rotator|MakeRotator 0.0 0.0 _rotation) false false))))
    (:B
      (bind _rotation_2 (Timeline|GoTiming PlayFromStart)
        (:Update
          (Transformation|SetRelativeRotation (Variables|Default|GetsquidGame_Doll_squidGameDoll_02_kepala) (Math|Rotator|MakeRotator 0.0 0.0 _rotation_2) false false))))))

(event EventTick
  (params (DeltaSeconds :type Float%20%28single-precision%29))
  ;[1 1 1] 회전 (2초부터 6초사이 랜덤 간격 )
  (Utilities|FlowControl|Delay (Math|Random|RandomFloatinRange 2.0 6.0))
  (CallFunction|Rotate180))

(fn ConstructionScript)
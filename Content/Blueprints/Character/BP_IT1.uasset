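; BP_IT1 is a "red light, green light" doll that plays the Mugungwa song and turns its head between phases.
; Tick drives a random 4–6 second Delay into Rotate180, whose FlipFlop alternates StopTiming and GoTiming timelines to rotate the head.
; Stopping pauses playing audio and sets RedLight when finished; going clears it and respawns the song afterward.
; During RedLight, Tick calls KillPlayer on any living player without checking movement here.
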(event Custom|Rotate180
  ;[1 1 1] 머리 회전
  (Utilities|FlowControl|FlipFlop
    (:A
      (if (Audio|Components|Audio|IsPlaying (Variables|Default|GetMugunghwa2D))
        (Class|AudioComponent|SetPaused (Variables|Default|GetMugunghwa2D) true)
        ;;[1 1 1] 회전 타이밍
        (bind _rotation (Timeline|StopTiming PlayFromStart)
          (:Update
            (Transformation|SetRelativeRotation (Variables|Default|Get123WoodManUpdated_DollHead) (Math|Rotator|MakeRotator 0.0 0.0 _rotation) false false))
          (:Finished
            (Variables|Default|SetRedLight true)))
        (else
          (Timeline|StopTiming PlayFromStart))))
    (:B
      (Variables|Default|SetRedLight false)
      (bind _rotation_2 (Timeline|GoTiming PlayFromStart)
        (:Update
          (Transformation|SetRelativeRotation (Variables|Default|Get123WoodManUpdated_DollHead) (Math|Rotator|MakeRotator 0.0 0.0 _rotation_2) false false))
        (:Finished
          (bind _returnvalue (Audio|SpawnSound2D "/Game/Sounds/Mugungwa_Cue.Mugungwa_Cue" 1.0 1.0 0.0 0))
          (Variables|Default|SetMugunghwa2D _returnvalue))))))

(event EventBeginPlay
  (bind _returnvalue (Audio|SpawnSound2D "/Game/Sounds/Mugungwa_Cue.Mugungwa_Cue" 1.0 1.0 0.0 0))
  (Variables|Default|SetMugunghwa2D _returnvalue)
  (bind _asbp_top_down_character (Utilities|Casting|CastToBP_TopDownCharacter (Game|GetPlayerCharacter 0)))
  (Variables|Default|SetPlayer _asbp_top_down_character))

(event EventTick
  (params (DeltaSeconds :type Float%20%28single-precision%29))
  (bind _player (Variables|Default|GetPlayer))
  (if (Variables|Default|GetRedLight)
    (if (Variables|/Game/Blueprints/Character/BP_TopDownCharacter.BP_TopDownCharacter_C|GetIsDead _player)
      ;[1 1 1] 회전 (4초부터 6초사이 랜덤 간격 )
      (Utilities|FlowControl|Delay (Math|Random|RandomFloatinRange 4.0 6.0) :!label _label)
      (CallFunction|Rotate180)
      (else
        (Default|KillPlayer _player)))
    (else
      (goto _label))))

(fn ConstructionScript)
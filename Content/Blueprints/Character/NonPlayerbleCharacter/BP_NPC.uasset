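; NPC contestant for a Red Light, Green Light game that moves forward until it dies or reaches the finish zone.
; Each tick, while IT is valid, it randomly nudges walk speed up on green or down on red within set limits.
; Light changes apply after a random reaction delay.
; KillPlayer marks unfinished NPCs still moving too fast as dead, then after a random delay plays a gunshot and enables physics.
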(event Custom|KillPlayer
  (if (not (or (Variables|Default|GetIsInFinishLine) (Variables|Default|GetIsDead)))
    (if (>= (Variables|/Script/Engine.CharacterMovementComponent|GetMaxWalkSpeed (Variables|Character|GetCharacterMovement)) 2e+01)
      (Variables|Default|SetIsDead true)
      (Utilities|FlowControl|Delay (Math|Random|RandomFloatinRange 0.0 1.5))
      (Audio|PlaySoundatLocation "/Game/Sounds/AK-47U/weap_akilo47_smg_plr_01_Cue.weap_akilo47_smg_plr_01_Cue" "0, 0, 0" "0, 0, 0" 1.0 1.0 0.0 0 0 0)
      (Physics|SetSimulatePhysics (Variables|Character|GetMesh) true))))

(event Custom|SetIT
  (params (IT :type BP%20IT1%20Object%20Reference))
  (Variables|Default|SetIT IT))

(event Custom|SetInFinishZone
  (params (IsIn :type Boolean))
  (Variables|Default|SetIsInFinishLine IsIn))

(event Custom|SetIT2
  (params (It2 :type BP%20IT2%20Object%20Reference))
  (Variables|Default|SetIT2 It2))

(event Custom|SetRedLight
  (params (RedLight :type Boolean))
  (Utilities|FlowControl|Delay (Math|Random|RandomFloatinRange 0.0 0.8))
  (Variables|Default|SetSplintMultiplier (Math|Random|RandomFloatinRange 1.0 3e+01))
  (Variables|Default|SetIsRedLight RedLight))

(event EventBeginPlay
  (Variables|/Script/Engine.CharacterMovementComponent|SetMaxWalkSpeed (Variables|Character|GetCharacterMovement) (Math|Random|RandomFloatinRange 1e+01 4e+02)))

(event EventTick
  (params (DeltaSeconds :type Float%20%28single-precision%29))
  (bind _movevalue (Variables|Default|GetMoveValue))
  (if (not (or (Variables|Default|GetIsDead) (Variables|Default|GetIsInFinishLine)))
    (Utilities|IsValid (Variables|Default|GetIT)
      (:Is%20Valid
        (if (Variables|Default|GetIsRedLight)
          (Variables|/Script/Engine.CharacterMovementComponent|SetMaxWalkSpeed (Variables|Character|GetCharacterMovement) (CallFunction|DecreaseMovementSpeed))
          (else
            (Variables|/Script/Engine.CharacterMovementComponent|SetMaxWalkSpeed (Variables|Character|GetCharacterMovement) (CallFunction|IncreaseMovementSpeed))))
        (Pawn|Input|AddMovementInput (* (Transformation|GetActorForwardVector) _movevalue) _movevalue false)))))

(fn ConstructionScript)

(fn IncreaseMovementSpeed
  (bind _output_get (Variables|Default|SetSplintMultiplier (Math|Random|RandomFloatinRange 0.3 1e+01)))
  (return (Math|Float|Clamp(Float) (+ (Variables|/Script/Engine.CharacterMovementComponent|GetMaxWalkSpeed (Variables|Character|GetCharacterMovement)) (Variables|Default|GetSplintMultiplier)) (Variables|Default|GetMinimumMovementSpeed) (Variables|Default|GetMaximumMovementSpeed))))

(fn DecreaseMovementSpeed
  (Variables|Default|SetSplintMultiplier (Math|Random|RandomFloatinRange 1.0 3e+01))
  (return (Math|Float|Clamp(Float) (- (Variables|/Script/Engine.CharacterMovementComponent|GetMaxWalkSpeed (Variables|Character|GetCharacterMovement)) (Variables|Default|GetSplintMultiplier)) (Variables|Default|GetMinimumMovementSpeed) (Variables|Default|GetMaximumMovementSpeed))))